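; Split-screen racing game mode that sets up two local players and runs the countdown to the race start.
; BeginPlay adds the second player; CreatePlayer gives each a possessed car, a per-screen HUD widget and the PlayerStart named by controller ID.
; Cars spawn with physics disabled.
; A looping timer plays countdown sounds, then StartRace adds each player's Enhanced Input mapping and enables car physics, so nobody moves early.
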(event Custom|StartRace
  (bind _outactors (Actor|GetAllActorsOfClass "/Script/Engine.PlayerController"))
  (for (_ _array_index) _outactors
    (Input|AddMappingContext (PlayerController|LocalPlayerSubsystems|GetEnhancedInputLocalPlayerSubsystem (Game|GetPlayerController _array_index)) "/Game/Inputs/IMC_Player.IMC_Player" 0 "(bIgnoreAllPressedKeysUntilRelease=True,bForceImmediately=False,bNotifyUserSettings=False)")
    (bind _asbp_player_car (Utilities|Casting|CastToBP_PlayerCar (Game|Player|GetPlayerPawn _array_index)))
    (Physics|SetSimulatePhysics (Variables|/Script/AstroRev.BaseCar|GetBaseCollider _asbp_player_car) true)))

(event Custom|CountTimer
  (bind _countdown (Variables|Default|GetCountdown))
  (Math|Integer|DecrementInt _countdown
    (:%20%20
      (if (< _countdown 0)
        (Utilities|Time|ClearandInvalidateTimerbyHandle (stale EventBeginPlay _returnvalue_2))
        (elif (== _countdown 0)
          (Audio|PlaySound2D "/Game/Sounds/SC_CountdownEnd.SC_CountdownEnd" 1.0 1.0 0.0 0 0)
          (CallFunction|StartRace)
          (else
            (Audio|PlaySound2D "/Game/Sounds/SC_Countdown.SC_Countdown" 1.0 1.0 0.0 0 0)))))))

(event EventBeginPlay
  (Utilities|FlowControl|Delay 0.2)
  (CallFunction|CreatePlayer (Game|GetPlayerController 0))
  (bind _returnvalue (Class|GameplayStatics|CreatePlayer -1))
  (CallFunction|CreatePlayer _returnvalue)
  (Audio|PlaySound2D "/Game/Sounds/Soundtrack/SC_MainMenu.SC_MainMenu" 1.0 1.0 0.0 0 0)
  (Utilities|FlowControl|Delay 2.0)
  (bind _returnvalue_2 (Utilities|Time|SetTimerbyEvent (delegate Custom|CountTimer) 1.0 true)))

(fn ConstructionScript)

(fn CreatePlayer
  (params (Player :type Player%20Controller%20Object%20Reference))
  (bind _returnvalue (Class|GameplayStatics|GetPlayerControllerID Player))
  (bind _returnvalue_2 (Game|SpawnActorfromClass "/Game/Blueprints/BP_PlayerCar.BP_PlayerCar_C" (Math|Transform|MakeTransform "0, 0, 0") "Undefined" "MultiplyWithRoot" 0 0))
  (Pawn|Possess Player _returnvalue_2)
  (bind _returnvalue_3 (UserInterface|CreateWidget "/Game/00-Blueprints/Widgets/W_Player.W_Player_C" Player))
  (Variables|/Game/Blueprints/BP_PlayerCar.BP_PlayerCar_C|SetW_Player _returnvalue_2 _returnvalue_3)
  (Variables|/Game/00-Blueprints/Widgets/W_Player.W_Player_C|SetPlayer _returnvalue_3 _returnvalue_2)
  (UserInterface|Viewport|AddtoPlayerScreen _returnvalue_3)
  (Physics|SetSimulatePhysics (Variables|/Script/AstroRev.BaseCar|GetBaseCollider _returnvalue_2) false)
  (Transformation|SetActorTransform _returnvalue_2 (Transformation|GetActorTransform (Class|GameModeBase|FindPlayerStart (Game|GetPlayerController _returnvalue) (Utilities|String|ToString(Integer) _returnvalue))) false true))