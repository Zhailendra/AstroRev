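; Game mode that drives layered audio which builds with the player car's speed.
; BeginPlay caches the BP_PlayerCar pawn and sets the base layer to full volume.
; Each Tick, SetLayerVolume sets four further layers from the car's speed as a fraction of MaxSpeed, minus a staggered per-layer threshold.
; The result is floored just above zero, so layers below their threshold stay barely audible rather than fully silent.
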(event EventBeginPlay
  (bind _asbp_player_car (Utilities|Casting|CastToBP_PlayerCar (Game|Player|GetPlayerPawn 0)))
  (Variables|Default|SetAs%20BP%20Player%20Car _asbp_player_car)
  (Audio|Components|Audio|SetVolumeMultiplier (Variables|Default|GetLayer0) 1.0 :!class /Script/Engine.AudioComponent))

(event EventTick
  (params (DeltaSeconds :type Float%20%28single-precision%29))
  (Utilities|IsValid (Variables|Default|GetAs%20BP%20Player%20Car)
    (:Is%20Valid
      (CallFunction|SetLayerVolume (Variables|Default|GetLayer1) 0.2)
      (CallFunction|SetLayerVolume (Variables|Default|GetLayer2) 0.4)
      (CallFunction|SetLayerVolume (Variables|Default|GetLayer3) 0.6)
      (CallFunction|SetLayerVolume (Variables|Default|GetLayer4) 0.8))))

(fn ConstructionScript)

(fn SetLayerVolume
  (params (Layer :type Audio%20Component%20Object%20Reference) (MinimumSpeed :type Float%20%28double-precision%29))
  (bind _as_bp_player_car (Variables|Default|GetAs%20BP%20Player%20Car))
  (Audio|Components|Audio|SetVolumeMultiplier Layer (Math|Float|Clamp(Float) (Math|Float|Max(Float) 0.01 (- (/ (Math|Vector|VectorLength (Transformation|GetVelocity _as_bp_player_car)) (/ (Variables|/Script/AstroRev.BaseCar|GetMaxSpeed _as_bp_player_car) 1.0)) MinimumSpeed))) :!class /Script/Engine.AudioComponent))