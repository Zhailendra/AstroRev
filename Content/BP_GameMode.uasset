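; BP_GameMode is a game mode with logic for layered audio that responds to the player car's speed, currently disconnected from its events.
; BeginPlay and Tick are empty, leaving the car-caching, base-layer and layer-update chains unreachable.
; SetLayerVolume sets a layer's volume from the car's speed as a fraction of MaxSpeed, minus that layer's threshold, clamped with a small floor.
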(event EventBeginPlay)

(event EventTick
  (params (DeltaSeconds :type Float%20%28single-precision%29)))

(fn ConstructionScript)

(fn SetLayerVolume
  (params (Layer :type Audio%20Component%20Object%20Reference) (MinimumSpeed :type Float%20%28double-precision%29))
  (bind _as_bp_player_car (Variables|Default|GetAs%20BP%20Player%20Car))
  (Audio|Components|Audio|SetVolumeMultiplier Layer (Math|Float|Clamp(Float) (Math|Float|Max(Float) 0.01 (- (/ (Math|Vector|VectorLength (Transformation|GetVelocity _as_bp_player_car)) (/ (Variables|/Script/AstroRev.BaseCar|GetMaxSpeed _as_bp_player_car) 1.0)) MinimumSpeed))) :!class /Script/Engine.AudioComponent))