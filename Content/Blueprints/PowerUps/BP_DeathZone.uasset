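; BP_DeathZone is a trigger volume that returns the player car to safety when it enters.
; Box overlap casts to BP_PlayerCar and targets its checkpoint if one is valid, otherwise its base location.
; One of two timelines moves the car there by lerping from its current location each update, with mesh physics simulation off during the move and restored when finished.
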(event OnComponentBeginOverlap(Box)
  (params (OverlappedComponent :type Primitive%20Component%20Object%20Reference) (OtherActor :type Actor%20Object%20Reference) (OtherComp :type Primitive%20Component%20Object%20Reference) (OtherBodyIndex :type Integer) (bFromSweep :type Boolean) (SweepResult :type Hit%20Result%20Structure%20%28by%20ref%29))
  (bind _asbp_player_car (Utilities|Casting|CastToBP_PlayerCar OtherActor))
  (Utilities|IsValid (Class|PlayerCar|GetCheckPoint _asbp_player_car)
    (:Is%20Valid
      (bind _newtrack_0 (Timeline|SmoothTeleport PlayFromStart)
        (:Update
          (Physics|SetSimulatePhysics (Variables|/Script/AstroRev.BaseCar|GetBaseMeshComponent _asbp_player_car) false)
          (Transformation|SetActorLocation _asbp_player_car (Math|Vector|Lerp(Vector) (Transformation|GetActorLocation _asbp_player_car) (Transformation|GetActorLocation (Class|PlayerCar|GetCheckPoint _asbp_player_car)) _newtrack_0) false false))
        (:Finished
          (Physics|SetSimulatePhysics (Variables|/Script/AstroRev.BaseCar|GetBaseMeshComponent _asbp_player_car) true))))
    (:Is%20Not%20Valid
      (bind _newtrack_0_2 (Timeline|Timeline PlayFromStart)
        (:Update
          (Physics|SetSimulatePhysics (Variables|/Script/AstroRev.BaseCar|GetBaseMeshComponent _asbp_player_car) false)
          (Transformation|SetActorLocation _asbp_player_car (Math|Vector|Lerp(Vector) (Transformation|GetActorLocation _asbp_player_car) (Class|PlayerCar|GetBaseLocation _asbp_player_car) _newtrack_0_2) false false))
        (:Finished
          (Physics|SetSimulatePhysics (Variables|/Script/AstroRev.BaseCar|GetBaseMeshComponent _asbp_player_car) true))))))

(event EventBeginPlay)

(event Collision|EventActorBeginOverlap
  (params (OtherActor :type Actor%20Object%20Reference)))

(event EventTick
  (params (DeltaSeconds :type Float%20%28single-precision%29)))

(fn ConstructionScript)